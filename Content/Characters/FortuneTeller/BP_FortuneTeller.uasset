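; Fortune teller character Blueprint that reacts with voice or sound and animation when the first tarot card is grabbed or released.
; Grabbing spawns the Heartbreak cue at the skeletal mesh and plays the Talk section of its montage; releasing stops the cue and plays Idle.
; Two DoOnce gates re-arm each other, so the Talk and Idle animations alternate rather than retrigger.
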(event `Grabbed_TarotCard_01`
  (bind _skeletalmesh (`self.SkeletalMesh`))
  (bind _returnvalue (`GameplayStatics.SpawnSoundAtLocation` "/Game/Sounds/Heartbreak_01_Cue.Heartbreak_01_Cue" (`SceneComponent.K2_GetComponentLocation` (`self.SkeletalMesh`)) (struct) 1.0 1.0 0.0 null null))
  (set `self.Sound_Heartbrake` _returnvalue)
  (`/Engine/EditorBlueprintResources/StandardMacros.DoOnce` false :!label _label
    (:`Completed`
      (`|PlayMontage` _skeletalmesh "/Game/Characters/FortuneTeller/FT_AnimMontage.FT_AnimMontage" 1.0 0.0 "Talk"
        (:`then`
          (goto _label_2 :!via `Reset`))))))

(event `Released_TarotCard_01`
  (`AudioComponent.Stop` (`self.Sound_Heartbrake`))
  (`/Engine/EditorBlueprintResources/StandardMacros.DoOnce` false :!label _label_2
    (:`Completed`
      (`|PlayMontage` (`self.SkeletalMesh`) "/Game/Characters/FortuneTeller/FT_AnimMontage.FT_AnimMontage" 1.0 0.0 "Idle"
        (:`then`
          (goto _label :!via `Reset`))))))

(fn `UserConstructionScript`)