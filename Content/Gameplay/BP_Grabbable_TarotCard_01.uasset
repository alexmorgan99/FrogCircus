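; Grabbable tarot card 01 that reports to the fortune teller when it is picked up or released.
; Grab disables physics and attaches the card to the given component, while Drop restores physics and detaches it, each notifying the first BP_FortuneTeller found.
; On destruction the card asks the Spawner cached at BeginPlay to spawn a card.
; Mesh overlaps toggle the actor's input for player 0.
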(event `self.StaticMeshComponent.OnComponentBeginOverlap`
  (params (OverlappedComponent :type "PrimitiveComponent Object Reference") (OtherActor :type "Actor Object Reference") (OtherComp :type "PrimitiveComponent Object Reference") (OtherBodyIndex :type Integer) (bFromSweep :type Boolean) (SweepResult :type "HitResult Structure (by ref)"))
  (`self.EnableInput` (`GameplayStatics.GetPlayerController` 0)))

(event `self.StaticMeshComponent.OnComponentEndOverlap`
  (params (OverlappedComponent :type "PrimitiveComponent Object Reference") (OtherActor :type "Actor Object Reference") (OtherComp :type "PrimitiveComponent Object Reference") (OtherBodyIndex :type Integer))
  (`self.DisableInput` (`GameplayStatics.GetPlayerController` 0)))

(event `/Game/BP_VR/BPI_GrabbableActor.Grab`
  (params (AttachTo :type "SceneComponent Object Reference"))
  (`PrimitiveComponent.SetSimulatePhysics` (`self.StaticMeshComponent`) false)
  (`SceneComponent.K2_AttachToComponent` (`self.RootComponent`) AttachTo "None" "KeepWorld" "KeepWorld" "KeepWorld" false)
  (bind _outactors (`GameplayStatics.GetAllActorsOfClass` "/Game/Characters/FortuneTeller/BP_FortuneTeller.BP_FortuneTeller_C"))
  (bind _asbp_fortune_teller (cast `/Game/Characters/FortuneTeller/BP_FortuneTeller` (`|GetArrayItem` _outactors)))
  (bind _output_get (set `self.FortuneTeller` _asbp_fortune_teller))
  (`/Game/Characters/FortuneTeller/BP_FortuneTeller.Grabbed_TarotCard_01` _output_get))

(event `/Game/BP_VR/BPI_GrabbableActor.Drop`
  (`PrimitiveComponent.SetSimulatePhysics` (`self.StaticMeshComponent`) true)
  (`self.K2_DetachFromActor` "KeepWorld" "KeepWorld" "KeepWorld")
  (bind _outactors (`GameplayStatics.GetAllActorsOfClass` "/Game/Characters/FortuneTeller/BP_FortuneTeller.BP_FortuneTeller_C"))
  (bind _asbp_fortune_teller (cast `/Game/Characters/FortuneTeller/BP_FortuneTeller` (`|GetArrayItem` _outactors)))
  (bind _output_get (set `self.FortuneTeller` _asbp_fortune_teller))
  (`/Game/Characters/FortuneTeller/BP_FortuneTeller.Released_TarotCard_01` _output_get))

(event `self.ReceiveBeginPlay`
  (bind _outactors (`GameplayStatics.GetAllActorsOfClass` "/Game/Gameplay/Spawner.Spawner_C"))
  (bind _asspawner (cast `/Game/Gameplay/Spawner` (`|GetArrayItem` _outactors)))
  (set `self.Spawner` _asspawner))

(event `self.ReceiveDestroyed`
  (`/Game/Gameplay/Spawner.SpawnCard` (`self.Spawner`)))

(fn `UserConstructionScript`)