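; Grabbable banana actor that splats on impact and respawns at a fixed spot.
; Grab turns off physics and attaches the root to the given component, while Drop restores physics and detaches it.
; A mesh hit plays a 2D splat sound, spawns a Niagara effect at the impact point, hides the actor and calls respawn with no delay.
; Respawn, also called on BeginPlay, moves the mesh to a hardcoded world location, disables physics and unhides the actor.
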(event `/Game/BP_VR/BPI_GrabbableActor.Grab`
  (params (AttachTo :type "SceneComponent Object Reference"))
  ;[1 1 1] Grab and Drop
  (`PrimitiveComponent.SetSimulatePhysics` (`self.StaticMeshComponent`) false)
  (`SceneComponent.K2_AttachToComponent` (`self.RootComponent`) AttachTo "None" "KeepWorld" "KeepWorld" "KeepWorld" false))

(event `Custom_Respawn`
  ;[1 1 1] Respawn
  (`SceneComponent.K2_SetWorldLocationAndRotation` :`self` (`self.StaticMeshComponent`) :`NewLocation` (682.628906 1395.001099 229.004364))
  (`PrimitiveComponent.SetSimulatePhysics` (`self.StaticMeshComponent`) false)
  (`self.SetActorHiddenInGame` false))

(event `/Game/BP_VR/BPI_GrabbableActor.Drop`
  ;[1 1 1] Grab and Drop
  (`PrimitiveComponent.SetSimulatePhysics` (`self.StaticMeshComponent`) true)
  (`self.K2_DetachFromActor` "KeepWorld" "KeepWorld" "KeepWorld"))

(event `self.ReceiveBeginPlay`
  ;[1 1 1] Respawn on Play
  (`self.Custom_Respawn`)
  (`self.SetActorHiddenInGame` false))

(event `Sound`
  (`GameplayStatics.PlaySound2D` "/Game/Sounds/splat_02.splat_02" 1.0 1.0 0.0 null null))

(event `self.StaticMeshComponent.OnComponentHit`
  (params (HitComponent :type "PrimitiveComponent Object Reference") (OtherActor :type "Actor Object Reference") (OtherComp :type "PrimitiveComponent Object Reference") (NormalImpulse :type "Vector Structure") (Hit :type "HitResult Structure (by ref)"))
  (`self.Sound`)
  (`NiagaraFunctionLibrary.SpawnSystemAtLocation` "/Game/FX/NS_Banana.NS_Banana" (`.ImpactPoint` (`GameplayStatics.BreakHitResult` Hit)))
  (`self.SetActorHiddenInGame` true)
  (`self.Custom_Respawn`))

(fn `UserConstructionScript`)